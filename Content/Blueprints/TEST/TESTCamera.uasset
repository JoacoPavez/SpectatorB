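; Test scene-capture camera actor that renders into an externally assigned render target.
; While ShouldUpdate is false, Tick pans the capture continuously in yaw and sways its pitch on a sine of elapsed time.
; Update snaps the root to a given PersonCharacter2's location, taking yaw from the actor and pitch from its FPS camera.
; Attach parents the actor to another, keeping relative transform.
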(event `self.ReceiveTick`
  (params (DeltaSeconds :type "Float (single-precision)"))
  (if (not (`self.ShouldUpdate`))
    (`self.Movement` DeltaSeconds)))

(fn `Attach`
  (params (Parent :type "Actor Object Reference"))
  (`self.K2_AttachToActor` self Parent "None" "KeepRelative" "KeepRelative" "KeepRelative" true))

(fn `Movement`
  (params (`Delta seconds` :type "Float (double-precision)"))
  (bind _scenecapture (`self.SceneCapture`))
  (bind (_returnvalue_roll _returnvalue_pitch _returnvalue_yaw) (`KismetMathLibrary.BreakRotator` (`SceneComponent.K2_GetComponentRotation` _scenecapture)))
  (bind _output_get (set `self.Time` (+ (`self.Time`) `Delta seconds`)))
  (`SceneComponent.K2_SetWorldRotation` _scenecapture (`KismetMathLibrary.MakeRotator` 0.0 (* 10 (`KismetMathLibrary.Lerp` -1.0 1.0 (`KismetMathLibrary.Sin` _output_get))) (+ _returnvalue_yaw (* 10 `Delta seconds`))) false false))

(fn `SetRender`
  (params (RenderTarget :type "CanvasRenderTarget2D Object Reference"))
  (set `SceneCaptureComponent2D.TextureTarget` RenderTarget (`self.SceneCapture`)))

(fn `Update`
  (params (Actor :type "Actor Object Reference"))
  (bind _asperson_character_2 (cast `/Game/Blueprints/PersonCharacter2` Actor))
  (`SceneComponent.K2_SetWorldLocationAndRotation` (`self.DefaultSceneRoot`) (`self.K2_GetActorLocation` Actor) (`KismetMathLibrary.MakeRotator` 0.0 (.pitch (`SceneComponent.K2_GetComponentRotation` (`/Game/Blueprints/PersonCharacter2.FPS_Camera` _asperson_character_2))) (.yaw (`self.K2_GetActorRotation` Actor))) false false))

(fn `UserConstructionScript`)