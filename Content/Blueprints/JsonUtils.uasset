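; JsonUtils is a Blueprint utility meant to save and load a SaveFile.json of player data.
; Its Loadfile, Savefile and Saveplayer events are empty, and the logic for them sits in disconnected chains that never run.
; Those chains read or write the JSON asynchronously, with an alternate synchronous load, and print results.
; The player chain adds or updates name, role and Y-value fields keyed by player index, then saves.
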(event `Load file`
  (params (`Screen prints` :type Boolean)))

(event `Save file`
  (params (`Screen prints` :type Boolean)))

(event `Save player`
  (params (Player :type "/Game/Blueprints/Blueprints/Player_Info Structure")))

(fn `UserConstructionScript`)