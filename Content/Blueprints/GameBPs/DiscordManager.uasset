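; Discord integration manager that posts messages to Discord channels and handles Discord lobbies and voice through a Discord Core created on BeginPlay.
; SendDiscordMessage looks up the channel ID in a data table, then creates a temporary webhook, executes it and deletes it.
; Lobby events create private, locked lobbies, store their IDs in an index-keyed map and connect by that key.
; ConnectVoice uses a hard-coded lobby ID and opens overlay voice settings, with debug prints throughout.
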(event `Send Discord Message`
  (params (Message :type String :default "Mensaje de prueba") (Channel :type Name :default "General") (ScreenPrints :type Boolean :default true) (Username :type String))
  ;[0.02459 1 0] Send Discord Message
  (`KismetSystemLibrary.PrintString` "Sending message to Discord..." ScreenPrints false (struct :`R` 1.0 :`G` 0.853695 :`A` 1.0))
  (bind _returnvalue (`|GetDataTableRow` "/Game/Blueprints/DataManagement/Channels.Channels" Channel)
    (:`then`
      (bind _newwebhoook (`CreateWebhookProxy.CreateWebhook` "Webhook1" "" (break `/Game/Blueprints/DataManagement/Channel` _returnvalue))
        (:`OnWebhookCreated`
          (bind (_id _type _guildid _channelid _user _name _avatar _token) (break `DiscordWebhook` _newwebhoook))
          (`ExecuteWebhookProxy.ExecuteWebhook` _id _token (make `DiscordWebhookData` Message Username)
            (:`OnWebhookExecuted`
              (`KismetSystemLibrary.PrintString` "Message sent!!" ScreenPrints false (struct :`R` 0.016251 :`G` 1.0 :`A` 1.0) 5.0)
              ;[1 0.8882 0] Modulo de borrado, es necesario?
              (`DeleteWebhookProxy.DeleteWebhook` _id
                (:`OnWebhookDeleted`
                  (`KismetSystemLibrary.PrintString` "Webhook deleted successfully!" ScreenPrints false (struct :`R` 0.016251 :`G` 1.0 :`A` 1.0) 5.0))
                (:`OnError`
                  (`KismetSystemLibrary.PrintString` "ERROR DELETING WEBHOOK" ScreenPrints false (struct :`R` 1.0 :`G` 0.013378 :`A` 1.0) 5.0))))))
        (:`OnError`
          (`KismetSystemLibrary.PrintString` "WEBHOOK ERROR" ScreenPrints false (struct :`R` 1.0 :`B` 0.029032 :`A` 1.0) 5.0)
          (bind (_id_2 _type_2 _guildid_2 _channelid_2 _user_2 _name_2) (break `DiscordWebhook` _newwebhoook))
          ;[1 0 0] Error de webhook
          (`KismetSystemLibrary.PrintString` (`KismetStringLibrary.Concat_StrStr` " \nID: " (`KismetStringLibrary.Conv_IntToString` (`KismetMathLibrary.Conv_Int64ToInt` _id_2)) " \nType: " (`|GetEnumeratorNameAsString` _type_2) " \nChannel ID: " (`KismetStringLibrary.Conv_IntToString` (`KismetMathLibrary.Conv_Int64ToInt` _channelid_2)) " \nUser: " _name_2) ScreenPrints false (struct :`R` 1.0 :`B` 0.029032 :`A` 1.0) 100.0))))))

(event `self.ReceiveBeginPlay`
  (set `self.DiscordCore` (`DiscordCore.CreateDiscordCore` "Default")))

(event `ConnectVoice`
  (bind _discordcore (`self.DiscordCore`))
  (`ConnectVoiceProxy.ConnectVoice` (`DiscordLobbyManager.GetLobbyManager` _discordcore) 861678837960146978
    (:`then`
      (`KismetSystemLibrary.PrintString` "TEST PRINT" true true (struct :`R` 0.958333 :`G` 0.868178 :`A` 1.0) 3.0))
    (:`OnSuccess`
      (`OpenVoiceSettingsProxy.OpenVoiceSettings` (`DiscordOverlayManager.GetOverlayManager` _discordcore)
        (:`OnSuccess`
          (`KismetSystemLibrary.PrintString` "Connected succesfully!" true true (struct :`G` 1.0 :`B` 0.055458 :`A` 1.0) 3.0))
        (:`OnError`
          (`KismetSystemLibrary.PrintString` "ERROR" true true (struct :`R` 1.0 :`G` 0.007248 :`A` 1.0) 5.0))))
    (:`OnError`
      (`KismetSystemLibrary.PrintString` "ERROR CONNECTING TO LOBBY" true true (struct :`R` 1.0 :`G` 0.007248 :`A` 1.0) 5.0))))

(event `Create Lobby`
  (bind _loobies (`self.Loobies`))
  (bind _discordcore (`self.DiscordCore`))
  (bind _returnvalue (`DiscordUserManager.GetUserManager` _discordcore))
  (bind _returnvalue_2 (`DiscordLobbyManager.GetLobbyManager` _discordcore))
  (bind _returnvalue_id (break `DiscordUser` (`DiscordUserManager.GetCurrentUser` _returnvalue)))
  (if (and (`KismetSystemLibrary.IsValid` _returnvalue_2) (`KismetSystemLibrary.IsValid` _returnvalue))
    (`KismetSystemLibrary.PrintString` (`KismetStringLibrary.Conv_IntToString` (`KismetMathLibrary.Conv_Int64ToInt` _returnvalue_id)))
    (bind _returnvalue_3 (`DiscordLobbyLibrary.SetLobbyTransactionProperties` (`DiscordLobbyManager.GetLobbyCreateTransaction` _returnvalue_2) "Private" (`|MakeMap` "Some key" "Some value") _returnvalue_id 10 true))
    (bind (_result _lobby) (`CreateLobbyProxy.CreateLobby` _returnvalue_2 _returnvalue_3)
      (:`then`
        (`BlueprintMapLibrary.Map_Add` _loobies (`BlueprintMapLibrary.Map_Length` _loobies) (break `DiscordLobby` _lobby))
        (`KismetSystemLibrary.PrintString` (`|GetEnumeratorNameAsString` _result))))))

(event `Connect to lobby`
  (params (`Lobby ID` :type Integer))
  (bind (_value _returnvalue) (`BlueprintMapLibrary.Map_Find` (`self.Loobies`) `Lobby ID`))
  (if _returnvalue
    (bind _result (`ConnectLobbyProxy.ConnectLobby` (`DiscordLobbyManager.GetLobbyManager` (`self.DiscordCore`)) _value)
      (:`then`
        (`KismetSystemLibrary.PrintString` (`|GetEnumeratorNameAsString` _result))))))

(fn `UserConstructionScript`)